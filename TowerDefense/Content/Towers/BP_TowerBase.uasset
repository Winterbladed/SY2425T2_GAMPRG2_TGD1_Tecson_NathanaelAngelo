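; Base tower actor for a tower defense game, with a range indicator, a clickable menu and selling.
; Range and menu start hidden, and clicking the tower passes it to its W_TowerMenu widget, then shows and focuses it.
; ShowRange scales the visual from the detector sphere's radius, while HideRange zeroes its scale.
; SellTower adds the sell cost as gold through the game mode and destroys the actor.
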(event `self.ReceiveBeginPlay`
  (`self.HideRange`)
  (`self.HideTowerMenu`))

(event `self.ReceiveTick`
  (params (DeltaSeconds :type "Float (single-precision)")))

(event `self.ReceiveActorOnClicked`
  (params (ButtonPressed :type "Key Structure"))
  (`self.ShowTowerMenu`)
  (`KismetSystemLibrary.PrintString` "tower clicked"))

(fn `HideRange`
  (`SceneComponent.SetWorldScale3D` (`self.RangeVisual`) (0.0 0.0 0.0)))

(fn `HideTowerMenu`
  (bind _asw_tower_menu (cast `/Game/Blueprints/W_TowerMenu` (`WidgetComponent.GetUserWidgetObject` (`self.TowerMenuWidget`))))
  (`Widget.SetVisibility` _asw_tower_menu "Collapsed"))

(fn `SellTower`
  (bind _returnvalue (`self.GetSellCost`))
  (bind _asbp_tower_defense_game_mode (cast `/Game/Blueprints/BP_TowerDefenseGameMode` (`GameplayStatics.GetGameMode`)))
  (`TowerDefenseCppGameModeBase.AddGold` _asbp_tower_defense_game_mode _returnvalue)
  (`self.K2_DestroyActor`))

(fn `ShowRange`
  (bind _returnvalue (/ (`SphereComponent.SphereRadius` (`self.RangeDetector`)) 50.0))
  (`SceneComponent.SetWorldScale3D` (`self.RangeVisual`) (`KismetMathLibrary.MakeVector` _returnvalue _returnvalue 1.0)))

(fn `ShowTowerMenu`
  (bind _asw_tower_menu (cast `/Game/Blueprints/W_TowerMenu` (`WidgetComponent.GetWidget` (`self.TowerMenuWidget`))))
  (`/Game/Blueprints/W_TowerMenu.SetTower` _asw_tower_menu (`self.TowerName`) self)
  (`Widget.SetUserFocus` _asw_tower_menu (`GameplayStatics.GetPlayerController` 0))
  (`Widget.SetVisibility` _asw_tower_menu "Visible"))

(fn `UserConstructionScript`)