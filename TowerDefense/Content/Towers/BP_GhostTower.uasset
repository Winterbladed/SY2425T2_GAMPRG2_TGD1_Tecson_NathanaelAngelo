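; BP_GhostTower is the tower placement preview, standing in for a real tower until it is placed on a platform.
; SetGhostTower maps the tower type to level-one Base and Head meshes (some types have no head mesh) and stores the matching Blueprint class.
; SetPlaceable tints the preview green or red.
; PlaceTower spawns the stored class at the platform's location, marks it occupied and destroys the ghost.
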(event `self.ReceiveTick`
  (params (DeltaSeconds :type "Float (single-precision)")))

(fn `PlaceTower`
  (params (Platform :type "/Game/Blueprints/BP_Platforms Object Reference"))
  (`/Engine/EditorBlueprintResources/StandardMacros.IsValid` Platform
    (:`Is Valid`
      (`|SpawnActorFromClass` (`self.TowerBlueprint`) (`KismetMathLibrary.MakeTransform` (`self.K2_GetActorLocation` Platform)) "AlwaysSpawn" "MultiplyWithRoot" null null)
      (set `/Game/Blueprints/BP_Platforms.isOccupied` true (`local.Platform`))
      (`self.K2_DestroyActor`)
      (return))))

(fn `SetGhostTower`
  (params (TowerType :type "/Game/Blueprints/E_TowerTypes Enum" :default "NewEnumerator0"))
  (switch `/Game/Blueprints/E_TowerTypes` TowerType
    (:`NewEnumerator0`
      (`StaticMeshComponent.SetStaticMesh` (`self.Base`) "/Game/Models/Base_MachineGun_L01.Base_MachineGun_L01")
      (`StaticMeshComponent.SetStaticMesh` (`self.Head`) "/Game/Models/Turret_MachineGun_L01.Turret_MachineGun_L01")
      (set `self.TowerBlueprint` "/Game/Towers/BP_Turret.BP_Turret_C"))
    (:`NewEnumerator1`
      (`StaticMeshComponent.SetStaticMesh` (`self.Base`) "/Game/Models/LaserTower_BASE_L01.LaserTower_BASE_L01")
      (`StaticMeshComponent.SetStaticMesh` (`self.Head`) "/Game/Models/LaserTower_TURRET_L01.LaserTower_TURRET_L01")
      (set `self.TowerBlueprint` "/Game/Towers/BP_LaserTower.BP_LaserTower_C"))
    (:`NewEnumerator2`
      (`StaticMeshComponent.SetStaticMesh` (`self.Base`) "/Game/Models/EMP_Tower_level_1.EMP_Tower_level_1")
      (`StaticMeshComponent.SetStaticMesh` (`self.Head`) null)
      (set `self.TowerBlueprint` "/Game/Towers/BP_EMP.BP_EMP_C"))
    (:`NewEnumerator3`
      (`StaticMeshComponent.SetStaticMesh` (`self.Base`) "/Game/Models/Base_RocketTower_L01.Base_RocketTower_L01")
      (`StaticMeshComponent.SetStaticMesh` (`self.Head`) "/Game/Models/Turret_RocketTower_L01.Turret_RocketTower_L01")
      (set `self.TowerBlueprint` "/Game/Towers/BP_MissileTower.BP_MissileTower_C"))
    (:`NewEnumerator4`
      (`StaticMeshComponent.SetStaticMesh` (`self.Base`) "/Game/Models/EnergyPylon_L01.EnergyPylon_L01")
      (`StaticMeshComponent.SetStaticMesh` (`self.Head`) null)
      (set `self.TowerBlueprint` "/Game/Towers/BP_Generator.BP_Generator_C"))
    (:`NewEnumerator5`
      (`StaticMeshComponent.SetStaticMesh` (`self.Base`) "/Game/Models/Salvager_L01.Salvager_L01")
      (`StaticMeshComponent.SetStaticMesh` (`self.Head`) null)
      (set `self.TowerBlueprint` "/Game/Towers/BP_Salvager.BP_Salvager_C"))))

(fn `SetPlaceable`
  (params (IsPlaceable :type Boolean))
  (bind _base (`self.Base`))
  (bind _head (`self.Head`))
  (bind _head_2 (`self.Head`))
  (if IsPlaceable
    (`PrimitiveComponent.SetMaterial` _base 0 "/Game/Blueprints/Green.Green")
    (`/Engine/EditorBlueprintResources/StandardMacros.IsValid` _head
      (:`Is Valid`
        (`PrimitiveComponent.SetMaterial` _head 0 "/Game/Blueprints/Green.Green")))
    (else
      (`PrimitiveComponent.SetMaterial` _base 0 "/Game/Blueprints/Red.Red")
      (`/Engine/EditorBlueprintResources/StandardMacros.IsValid` _head_2
        (:`Is Valid`
          (`PrimitiveComponent.SetMaterial` _head_2 0 "/Game/Blueprints/Red.Red"))))))

(fn `UserConstructionScript`)