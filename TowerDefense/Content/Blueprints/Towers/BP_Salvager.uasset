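; BP_Salvager is an economy tower that earns passive gold and boosts gold drops from nearby enemies.
; A looping timer periodically adds its truncated special value to the tower defense game mode's gold.
; Every Tick it sets that same value as the bonus drop on enemies overlapping RangeDetector.
; The bonus is set rather than added, and resets to zero when an enemy leaves range or the tower is destroyed.
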(event `self.ReceiveBeginPlay`
  (`parent.ReceiveBeginPlay`)
  (`KismetSystemLibrary.K2_SetTimerDelegate` (delegate `GainPassiveGold`) 3.0 true))

(event `GainPassiveGold`
  (bind _asbp_tower_defense_game_mode (cast `/Game/Blueprints/BP_TowerDefenseGameMode` (`GameplayStatics.GetGameMode`)))
  (bind _returnvalue (`self.GetSpecialValue`))
  (`TowerDefenseCppGameModeBase.AddGold` _asbp_tower_defense_game_mode (`KismetMathLibrary.FTrunc` _returnvalue)))

(event `self.ReceiveTick`
  (params (DeltaSeconds :type "Float (single-precision)"))
  (`parent.ReceiveTick` DeltaSeconds)
  (for _array_element (`PrimitiveComponent.GetOverlappingActors` (`self.RangeDetector`) "/Game/Blueprints/Enemies/BP_EnemyBase.BP_EnemyBase_C")
    (bind _asbp_enemy_base (cast `/Game/Blueprints/Enemies/BP_EnemyBase` _array_element))
    (bind _returnvalue (`self.GetSpecialValue`))
    (`Enemy.SetBonusGoldDrop` _asbp_enemy_base _returnvalue)))

(event `self.RangeDetector.OnComponentEndOverlap`
  (params (OverlappedComponent :type "PrimitiveComponent Object Reference") (OtherActor :type "Actor Object Reference") (OtherComp :type "PrimitiveComponent Object Reference") (OtherBodyIndex :type Integer))
  (bind _asbp_enemy_base (cast `/Game/Blueprints/Enemies/BP_EnemyBase` OtherActor))
  (`Enemy.SetBonusGoldDrop` _asbp_enemy_base 0.0))

(event `self.ReceiveDestroyed`
  (for _array_element (`PrimitiveComponent.GetOverlappingActors` (`self.RangeDetector`) "/Game/Blueprints/Enemies/BP_EnemyBase.BP_EnemyBase_C")
    (bind _asbp_enemy_base (cast `/Game/Blueprints/Enemies/BP_EnemyBase` _array_element))
    (`Enemy.SetBonusGoldDrop` _asbp_enemy_base 0.0)))

(fn `UserConstructionScript`
  (`parent.UserConstructionScript`))