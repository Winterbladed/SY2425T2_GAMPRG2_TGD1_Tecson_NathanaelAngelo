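; Base buff actor that runs for a limited duration, with empty ActionEvent as a hook for a specific effect.
; Tick counts Duration down; on expiry OnDeactivate calls the Deactivate dispatcher and destroys the actor.
; OnActivate starts a looping timer for periodic actions when ActionInterval is positive.
; ResetTimer restores the duration saved at BeginPlay, refreshing the buff.
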(event `self.ReceiveBeginPlay`
  (set `self.OriginalDuration` (`self.Duration`)))

(event `self.ReceiveTick`
  (params (DeltaSeconds :type "Float (single-precision)"))
  (if (> (`self.Duration`) 0.0)
    (bind _output_get (set `self.Duration` (- (`self.Duration`) DeltaSeconds)))
    (if (<= _output_get 0.0)
      (`self.OnDeactivate`))))

(fn `ActionEvent`)

(fn `OnActivate`
  (if (> (`self.ActionInterval`) 0.0)
    (`KismetSystemLibrary.K2_SetTimerDelegate` (`|CreateDelegate` :!event `ActionEvent`) (`self.ActionInterval`) true)))

(fn `OnDeactivate`
  (`self.Deactivate` self)
  (`self.K2_DestroyActor`))

(fn `ResetTimer`
  (set `self.Duration` (`self.OriginalDuration`)))

(fn `UserConstructionScript`)