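; Actor component, going by its AC_ prefix, that tracks the active buff actors applied to its owner.
; ReceiveBuff resets the timer of any same-class buff and destroys the incoming duplicate; a new class is stored, given a handler reference and activated.
; It also binds an event to each new buff's deactivation.
; DeactivateBuff calls OnDeactivate on buffs of a given class, while RemoveBuff drops one from the list.
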(fn `DeactivateBuff`
  (params (Buff :type "/Game/Blueprints/Buffs/BP_Buff Class Reference"))
  (for _array_element (`self.Buffs`)
    (if (== (`GameplayStatics.GetObjectClass` _array_element) Buff)
      (`/Game/Blueprints/Buffs/BP_Buff.OnDeactivate` _array_element))))

(fn `ReceiveBuff`
  (params (BuffClass :type "/Game/Blueprints/Buffs/BP_Buff Object Reference"))
  (locals (HasBuff :type Boolean))
  (for _array_element (`self.Buffs`)
    (if (== (`GameplayStatics.GetObjectClass` _array_element) (`GameplayStatics.GetObjectClass` BuffClass))
      (set `local.HasBuff` true)
      (`/Game/Blueprints/Buffs/BP_Buff.ResetTimer` _array_element)
      (`Actor.K2_DestroyActor` BuffClass)))
  (if (not (`local.HasBuff`))
    (`KismetArrayLibrary.Array_Add` (`self.Buffs`) BuffClass)
    (add `/Game/Blueprints/Buffs/BP_Buff.Deactivate` BuffClass (`|CreateDelegate` :!event `RemoveBuff`))
    (set `/Game/Blueprints/Buffs/BP_Buff.Handler` self BuffClass)
    (`/Game/Blueprints/Buffs/BP_Buff.OnActivate` BuffClass)))

(fn `RemoveBuff`
  (params (Buff :type "/Game/Blueprints/Buffs/BP_Buff Object Reference"))
  (`KismetArrayLibrary.Array_RemoveItem` (`self.Buffs`) Buff))