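; Overload buff that modifies a tower's attack rate while active.
; On activation it finds the BP_TowerBase that owns its Handler and divides that tower's FireRate by BoostAmount; deactivation multiplies it back.
; SetAttackRateModifier supplies BoostAmount, which is not cached per activation, so changing it mid-buff skews the restored rate.
; Parent activate and deactivate logic runs only when the Handler and tower cast are valid.
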(fn `OnActivate`
  (bind _handler (`self.Handler`))
  (`/Engine/EditorBlueprintResources/StandardMacros.IsValid` _handler
    (:`Is Valid`
      (bind _asbp_tower_base (cast `/Game/Blueprints/Towers/BP_TowerBase` (`ActorComponent.GetOwner` _handler)))
      (bind _returnvalue (`Tower.GetFireRate` _asbp_tower_base))
      (`Tower.SetFireRate` _asbp_tower_base (/ _returnvalue (`self.BoostAmount`)))
      (`parent.OnActivate`))))

(fn `OnDeactivate`
  (bind _handler (`self.Handler`))
  (`/Engine/EditorBlueprintResources/StandardMacros.IsValid` _handler
    (:`Is Valid`
      (bind _asbp_tower_base (cast `/Game/Blueprints/Towers/BP_TowerBase` (`ActorComponent.GetOwner` _handler)))
      (bind _returnvalue (`Tower.GetFireRate` _asbp_tower_base))
      (`Tower.SetFireRate` _asbp_tower_base (* _returnvalue (`self.BoostAmount`)))
      (`parent.OnDeactivate`))))

(fn `SetAttackRateModifier`
  (params (AttackRateBoost :type "Float (double-precision)"))
  (set `self.BoostAmount` AttackRateBoost))

(fn `UserConstructionScript`
  (`parent.UserConstructionScript`))