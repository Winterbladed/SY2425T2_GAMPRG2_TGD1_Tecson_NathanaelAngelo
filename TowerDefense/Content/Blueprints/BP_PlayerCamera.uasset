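; Player camera Blueprint that places its Camera at preset transforms stored in the CameraSettingsA array.
; BeginPlay resets CameraIndex to 0 and applies that preset through SetCameraLocation, which sets the camera's world transform directly.
; Space Bar picks preset 1 or 0 based on CameraIndex, but nothing here changes the index after BeginPlay, so it reapplies preset 0.
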(event `self.ReceiveBeginPlay`
  (bind _output_get (set `self.CameraIndex` 0))
  (`self.SetCameraLocation` _output_get))

(event `Key|SpaceBar`
  (params (Key :type "Key Structure"))
  (:`Pressed`
    (if (!= 0 (`self.CameraIndex`))
      (`self.SetCameraLocation` 1)
      (else
        (`self.SetCameraLocation` 0)))))

(fn `SetCameraLocation`
  (params (Index :type Integer))
  (`SceneComponent.K2_SetWorldTransform` (`self.Camera`) (`|GetArrayItem` (`self.CameraSettingsA`) Index) false false))

(fn `UserConstructionScript`)