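; Player controller for a tower defense game that handles mouse-driven tower placement with a ghost preview.
; Each tick, a cursor trace against WorldStatic moves the ghost and marks it placeable only over an unoccupied BP_Platforms, which becomes the target node.
; Left click places the tower on that node and deducts its cost through BP_TowerDefenseGameMode; right click destroys the ghost.
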(event `self.ReceiveTick`
  (params (DeltaSeconds :type "Float (single-precision)"))
  (bind _ghosttowerref (`self.GhostTowerRef`))
  (bind _ghosttowerref_2 (`self.GhostTowerRef`))
  (bind (_hitresult _returnvalue) (`self.GetHitResultUnderCursorForObjects` (`|MakeArray` "ObjectTypeQuery1" :!type "EObjectTypeQuery Enum")))
  (bind (_bblockinghit _binitialoverlap _time _distance _location _impactpoint _normal _impactnormal _physmat _hitactor) (`GameplayStatics.BreakHitResult` _hitresult))
  (if _returnvalue
    (`/Engine/EditorBlueprintResources/StandardMacros.IsValid` _ghosttowerref
      (:`Is Valid`
        (`SceneComponent.K2_SetWorldLocation` (`Actor.RootComponent` _ghosttowerref) _location false false)
        (bind _asbp_platforms (cast `/Game/Blueprints/BP_Platforms` _hitactor)
          (:`then`
            (if (`/Game/Blueprints/BP_Platforms.isOccupied` _asbp_platforms)
              (set `self.TowerNode` null)
              (`/Game/Towers/BP_GhostTower.SetPlaceable` _ghosttowerref_2 false)
              (set `self.IsTowerPlaceable` false)
              (else
                (set `self.TowerNode` _asbp_platforms)
                (`/Game/Towers/BP_GhostTower.SetPlaceable` _ghosttowerref_2 true)
                (set `self.IsTowerPlaceable` true))))
          (:`CastFailed`
            (`/Game/Towers/BP_GhostTower.SetPlaceable` _ghosttowerref false)
            (set `self.IsTowerPlaceable` false)))))))

(event `Key|LeftMouseButton`
  (params (Key :type "Key Structure"))
  (:`Pressed`
    (if (`self.IsTowerPlaceable`)
      (`/Game/Towers/BP_GhostTower.PlaceTower` (`self.GhostTowerRef`) (`self.TowerNode`))
      (bind _asbp_tower_defense_game_mode (cast `/Game/Blueprints/BP_TowerDefenseGameMode` (`GameplayStatics.GetGameMode`)))
      (`TowerDefenseCppGameModeBase.DeductGold` _asbp_tower_defense_game_mode (`self.GhostTowerCost`))
      (set `self.TowerNode` null)
      (set `self.IsTowerPlaceable` false))))

(event `Key|RightMouseButton`
  (params (Key :type "Key Structure"))
  (bind _ghosttowerref (`self.GhostTowerRef`))
  (:`Pressed`
    (`/Engine/EditorBlueprintResources/StandardMacros.IsValid` _ghosttowerref
      (:`Is Valid`
        (`self.K2_DestroyActor` _ghosttowerref)))))

(fn `UserConstructionScript`)