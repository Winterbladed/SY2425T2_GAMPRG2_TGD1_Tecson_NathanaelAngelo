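; BP_NormalBullet is a short-lived projectile that damages enemies on overlap.
; It passes its Damage to the EnemyHealthComponent of any BP_EnemyBase it touches, then destroys itself.
; Overlaps with Projectile or Tower actors are ignored, while any other actor destroys the bullet.
; A delay started on BeginPlay removes bullets that hit nothing.
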(event `self.ReceiveBeginPlay`
  (`KismetSystemLibrary.Delay` 2.0)
  (`self.K2_DestroyActor`))

(event `self.ReceiveActorBeginOverlap`
  (params (OtherActor :type "Actor Object Reference"))
  (bind _asbp_enemy_base (cast `/Game/Blueprints/Enemies/BP_EnemyBase` OtherActor)
    (:`then`
      (`HealthComponent.TakeDamage` (`Enemy.EnemyHealthComponent` _asbp_enemy_base) (`self.Damage`))
      (`self.K2_DestroyActor`))
    (:`CastFailed`
      (cast `Projectile` OtherActor
        (:`CastFailed`
          (cast `Tower` OtherActor
            (:`CastFailed`
              (`self.K2_DestroyActor`))))))))

(fn `UserConstructionScript`)