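; Burn debuff that deals damage to the enemy it is attached to.
; SetBurnDamage stores the damage amount, passed in as DPS, and sets a fixed five-second duration.
; ActionEvent casts the valid Handler's owner to BP_EnemyBase and applies that damage through its EnemyHealthComponent.
; The file contains no timing logic of its own, and its event graph holds only disabled stubs.
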(fn `ActionEvent`
  (bind _handler (`self.Handler`))
  (`/Engine/EditorBlueprintResources/StandardMacros.IsValid` _handler
    (:`Is Valid`
      (bind _asbp_enemy_base (cast `/Game/Enemies/BP_EnemyBase` (`ActorComponent.GetOwner` _handler)))
      (`HealthComponent.TakeDamage` (`Enemy.EnemyHealthComponent` _asbp_enemy_base) (`self.BurnDamage`)))))

(fn `SetBurnDamage`
  (params (DPS :type "Float (double-precision)"))
  (set `self.BurnDamage` DPS)
  (set `self.Duration` 5.0))

(fn `UserConstructionScript`
  (`parent.UserConstructionScript`))