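; BP_EnemyBase is an enemy base Blueprint that keeps a health bar widget in sync with the enemy's health.
; Every Tick, UpdateHealthBar casts the HealthBar component's user widget to W_EnemyHealthBar and copies current and max HP into it from EnemyHealthComponent.
; The bar updates by per-frame polling, and BeginPlay and the construction script are empty.
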(event `self.ReceiveBeginPlay`)

(event `self.ReceiveTick`
  (params (DeltaSeconds :type "Float (single-precision)"))
  (`self.UpdateHealthBar`))

(fn `UpdateHealthBar`
  (bind _asw_enemy_health_bar (cast `/Game/Blueprints/W_EnemyHealthBar` (`WidgetComponent.GetUserWidgetObject` (`self.HealthBar`))))
  (bind _returnvalue (`HealthComponent.GetCurrentHp` (`self.EnemyHealthComponent`)))
  (set `/Game/Blueprints/W_EnemyHealthBar.CurrentHp` _returnvalue _asw_enemy_health_bar)
  (bind _returnvalue_2 (`HealthComponent.GetMaxHp` (`self.EnemyHealthComponent`)))
  (set `/Game/Blueprints/W_EnemyHealthBar.MaxHp` _returnvalue_2 _asw_enemy_health_bar))

(fn `UserConstructionScript`)