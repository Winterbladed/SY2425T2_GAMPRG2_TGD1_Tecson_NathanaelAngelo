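; BP_Missile is a projectile that deals area damage to ground enemies when it hits something.
; On a hit of its ProjectileMesh, it sizes a Sphere component to SpecialValue and gathers the overlapping BP_EnemyBase actors.
; Each one flagged as a ground enemy takes Damage through its EnemyHealthComponent, with a debug print.
; The missile then destroys itself.
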(event `self.ProjectileMesh.OnComponentHit`
  (params (HitComponent :type "PrimitiveComponent Object Reference") (OtherActor :type "Actor Object Reference") (OtherComp :type "PrimitiveComponent Object Reference") (NormalImpulse :type "Vector Structure") (Hit :type "HitResult Structure (by ref)"))
  (`SceneComponent.SetWorldScale3D` (`self.Sphere`) (1.0 1.0 1.0))
  (`SphereComponent.SetSphereRadius` (`self.Sphere`) (`self.SpecialValue`) true)
  (for _array_element (`PrimitiveComponent.GetOverlappingActors` (`self.Sphere`) "/Game/Enemies/BP_EnemyBase.BP_EnemyBase_C")
    (bind _asbp_enemy_base (cast `/Game/Enemies/BP_EnemyBase` _array_element))
    (if (`/Game/Enemies/BP_EnemyBase.IsGroundEnemy` _asbp_enemy_base)
      (`HealthComponent.TakeDamage` (`Enemy.EnemyHealthComponent` _asbp_enemy_base) (`self.Damage`))
      (`KismetSystemLibrary.PrintString` "Missile")))
  (`self.K2_DestroyActor`))

(fn `UserConstructionScript`)