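; BP_EMP is a tower that slows enemies inside its range.
; When a BP_EnemyBase enters RangeDetector, it spawns a BP_SlowDebuff, sets its slow percent from GetSpecialValue and hands it to the enemy's BuffHandler.
; Leaving the range deactivates that debuff class on the enemy, and destroying the tower does the same for every enemy still overlapping.
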(event `self.ReceiveTick`
  (params (DeltaSeconds :type "Float (single-precision)"))
  (`parent.ReceiveTick` DeltaSeconds))

(event `self.RangeDetector.OnComponentBeginOverlap`
  (params (OverlappedComponent :type "PrimitiveComponent Object Reference") (OtherActor :type "Actor Object Reference") (OtherComp :type "PrimitiveComponent Object Reference") (OtherBodyIndex :type Integer) (bFromSweep :type Boolean) (SweepResult :type "HitResult Structure (by ref)"))
  (bind _asbp_enemy_base (cast `/Game/Enemies/BP_EnemyBase` OtherActor))
  (bind _returnvalue (`|SpawnActorFromClass` "/Game/Buffs/BP_SlowDebuff.BP_SlowDebuff_C" (`KismetMathLibrary.MakeTransform` (0.0 0.0 0.0)) "AlwaysSpawn" "MultiplyWithRoot" null null))
  (bind _returnvalue_2 (`self.GetSpecialValue`))
  (`/Game/Buffs/BP_SlowDebuff.SetSlowPercent` _returnvalue _returnvalue_2)
  (`/Game/Blueprints/AC_BuffHandler.ReceiveBuff` (`/Game/Enemies/BP_EnemyBase.BuffHandler` _asbp_enemy_base) _returnvalue))

(event `self.RangeDetector.OnComponentEndOverlap`
  (params (OverlappedComponent :type "PrimitiveComponent Object Reference") (OtherActor :type "Actor Object Reference") (OtherComp :type "PrimitiveComponent Object Reference") (OtherBodyIndex :type Integer))
  (bind _asbp_enemy_base (cast `/Game/Enemies/BP_EnemyBase` OtherActor))
  (`/Game/Blueprints/AC_BuffHandler.DeactivateBuff` (`/Game/Enemies/BP_EnemyBase.BuffHandler` _asbp_enemy_base) "/Game/Buffs/BP_SlowDebuff.BP_SlowDebuff_C"))

(event `self.ReceiveDestroyed`
  (for _array_element (`PrimitiveComponent.GetOverlappingActors` (`self.RangeDetector`) "/Game/Enemies/BP_EnemyBase.BP_EnemyBase_C")
    (bind _asbp_enemy_base (cast `/Game/Enemies/BP_EnemyBase` _array_element))
    (`/Game/Blueprints/AC_BuffHandler.DeactivateBuff` (`/Game/Enemies/BP_EnemyBase.BuffHandler` _asbp_enemy_base) "/Game/Buffs/BP_SlowDebuff.BP_SlowDebuff_C")))

(fn `UserConstructionScript`
  (`parent.UserConstructionScript`))