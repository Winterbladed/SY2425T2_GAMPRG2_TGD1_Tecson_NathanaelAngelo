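; BP_SlowDebuff is a buff that slows an enemy while active.
; On activation it casts the handler's owner to BP_EnemyBase and multiplies its FloatingPawnMovement max speed by SlowPercent.
; On deactivation it divides the current max speed by SlowPercent to undo the slow, relying on the value staying unchanged in between.
; SetSlowPercent sets that factor, and parent activation logic runs only after a successful cast.
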(fn `OnActivate`
  (bind _handler (`self.Handler`))
  (`/Engine/EditorBlueprintResources/StandardMacros.IsValid` _handler
    (:`Is Valid`
      (bind _asbp_enemy_base (cast `/Game/Blueprints/Enemies/BP_EnemyBase` (`ActorComponent.GetOwner` _handler)))
      (bind _floatingpawnmovement (`/Game/Blueprints/Enemies/BP_EnemyBase.FloatingPawnMovement` _asbp_enemy_base))
      (set `FloatingPawnMovement.MaxSpeed` (* (`MovementComponent.GetMaxSpeed` _floatingpawnmovement) (`self.SlowPercent`)) _floatingpawnmovement)
      (`parent.OnActivate`))))

(fn `OnDeactivate`
  (bind _handler (`self.Handler`))
  (`/Engine/EditorBlueprintResources/StandardMacros.IsValid` _handler
    (:`Is Valid`
      (bind _asbp_enemy_base (cast `/Game/Blueprints/Enemies/BP_EnemyBase` (`ActorComponent.GetOwner` _handler)))
      (bind _floatingpawnmovement (`/Game/Blueprints/Enemies/BP_EnemyBase.FloatingPawnMovement` _asbp_enemy_base))
      (set `FloatingPawnMovement.MaxSpeed` (/ (`MovementComponent.GetMaxSpeed` _floatingpawnmovement) (`self.SlowPercent`)) _floatingpawnmovement)
      (`parent.OnDeactivate`))))

(fn `SetSlowPercent`
  (params (SlowPercentAmount :type "Float (double-precision)"))
  (set `self.SlowPercent` SlowPercentAmount))

(fn `UserConstructionScript`
  (`parent.UserConstructionScript`))