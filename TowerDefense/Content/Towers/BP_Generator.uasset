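; BP_Generator is a support tower that applies an attack-rate overload buff to towers within its RangeDetector.
; Every tick it spawns a new BP_OverloadBuff actor for each overlapping tower, sets its modifier from GetSpecialValue and passes it to that tower's TowerBuffHandler.
; When destroyed, it deactivates the overload buff class on towers still in range.
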(event `self.ReceiveTick`
  (params (DeltaSeconds :type "Float (single-precision)"))
  (`parent.ReceiveTick` DeltaSeconds)
  (for _array_element (`PrimitiveComponent.GetOverlappingActors` (`self.RangeDetector`) "/Game/Towers/BP_TowerBase.BP_TowerBase_C")
    (bind _asbp_tower_base (cast `/Game/Towers/BP_TowerBase` _array_element))
    (bind _returnvalue (`|SpawnActorFromClass` "/Game/Buffs/BP_OverloadBuff.BP_OverloadBuff_C" (`KismetMathLibrary.MakeTransform` (0.0 0.0 0.0)) "AlwaysSpawn" "MultiplyWithRoot" null null))
    (bind _returnvalue_2 (`self.GetSpecialValue`))
    (`/Game/Buffs/BP_OverloadBuff.SetAttackRateModifier` _returnvalue _returnvalue_2)
    (`/Game/Blueprints/AC_BuffHandler.ReceiveBuff` (`/Game/Towers/BP_TowerBase.TowerBuffHandler` _asbp_tower_base) _returnvalue)))

(event `self.ReceiveDestroyed`
  (for _array_element (`PrimitiveComponent.GetOverlappingActors` (`self.RangeDetector`) "/Game/Towers/BP_TowerBase.BP_TowerBase_C")
    (bind _asbp_tower_base (cast `/Game/Towers/BP_TowerBase` _array_element))
    (`/Game/Blueprints/AC_BuffHandler.DeactivateBuff` (`/Game/Towers/BP_TowerBase.TowerBuffHandler` _asbp_tower_base) "/Game/Buffs/BP_OverloadBuff.BP_OverloadBuff_C")))

(fn `UserConstructionScript`
  (`parent.UserConstructionScript`))